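; BP_Lift is a lift that the player raises and lowers with Left Shift while in its trigger box.
; The Box overlap events enable and disable input for player controller 0, without checking which actor overlaps.
; Each press prints a debug "Hello" and flip-flops the LiftOperastor timeline between play and reverse.
; The timeline's Height track, scaled by a fixed distance, sets the Lift component's relative Z.
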(event `self.Box.OnComponentBeginOverlap`
  (params (OverlappedComponent :type "PrimitiveComponent Object Reference") (OtherActor :type "Actor Object Reference") (OtherComp :type "PrimitiveComponent Object Reference") (OtherBodyIndex :type Integer) (bFromSweep :type Boolean) (SweepResult :type "HitResult Structure (by ref)"))
  (`self.EnableInput` (`GameplayStatics.GetPlayerController` 0)))

(event `self.Box.OnComponentEndOverlap`
  (params (OverlappedComponent :type "PrimitiveComponent Object Reference") (OtherActor :type "Actor Object Reference") (OtherComp :type "PrimitiveComponent Object Reference") (OtherBodyIndex :type Integer))
  (`self.DisableInput` (`GameplayStatics.GetPlayerController` 0)))

(event `Key|LeftShift`
  (params (Key :type "Key Structure"))
  (:`Pressed`
    (`KismetSystemLibrary.PrintString` "Hello")
    (`/Engine/EditorBlueprintResources/StandardMacros.FlipFlop`
      (:`A`
        (bind (_direction _height) (`Timeline|Lift Operastor` :!label _label)
          (:`Update`
            (`SceneComponent.K2_SetRelativeLocation` (`self.Lift`) (`KismetMathLibrary.MakeVector` 0.0 0.0 (* _height 500.0)) false false))))
      (:`B`
        (goto _label :!via `Reverse`)))))

(fn `UserConstructionScript`)