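; BP_ChargeHolder is a socket actor that detects an inserted BP_singleCharge and signals the change, apparently for opening a door.
; When a charge enters its Box, it stores the reference, sets IsTriggered and fires the ChargeInserted dispatcher.
; When the last charge leaves, it clears IsTriggered and fires ChargeRemoved.
; Both changes print colored door status messages; any door logic lives outside this Blueprint.
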(event `self.Box.OnComponentBeginOverlap`
  (params (OverlappedComponent :type "PrimitiveComponent Object Reference") (OtherActor :type "Actor Object Reference") (OtherComp :type "PrimitiveComponent Object Reference") (OtherBodyIndex :type Integer) (bFromSweep :type Boolean) (SweepResult :type "HitResult Structure (by ref)"))
  (bind _asbp_single_charge (cast `/Game/Blueprints/BP_singleCharge` OtherActor))
  (set `self.Charge` _asbp_single_charge)
  (set `self.isTriggered?` true)
  (`self.Charge_Inserted`)
  (`KismetSystemLibrary.PrintString` "Door Open" true true (struct :`G` 1.0 :`B` 0.134427 :`A` 1.0) 3.0))

(event `self.Box.OnComponentEndOverlap`
  (params (OverlappedComponent :type "PrimitiveComponent Object Reference") (OtherActor :type "Actor Object Reference") (OtherComp :type "PrimitiveComponent Object Reference") (OtherBodyIndex :type Integer))
  (if (`KismetArrayLibrary.Array_IsEmpty` (`PrimitiveComponent.GetOverlappingActors` (`self.Box`) "/Game/Blueprints/BP_singleCharge.BP_singleCharge_C"))
    (set `self.isTriggered?` false)
    (`self.Charge_Removed`)
    (`KismetSystemLibrary.PrintString` "eccess denied" true true (struct :`R` 1.0 :`B` 0.102586 :`A` 1.0) 3.0)))

(fn `UserConstructionScript`)